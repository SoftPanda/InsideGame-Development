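; Interior door actor for the Old Brick House that swings its mesh open and closed when the MoveDoor event is called.
; MoveDoor plays the DoorMovement timeline while its AxisZ value is below 1.0 and reverses it otherwise.
; Each timeline update sets the mesh's relative yaw to AxisZ, or to 1.0 minus AxisZ, depending on IsOpeningInwards to choose the swing direction.
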(event Custom|Move%20Door
  (bind _sm_oldbrickhouse_door_interior_01 (Variables|Default|GetSM_OldBrickHouse_Door_Interior_01))
  (if (< (stale _axisz) 1.0)
    (bind _axisz (Timeline|doorMovement Play)
      (:Update
        (if (Variables|Default|GetisOpeningInwards)
          (Transformation|SetRelativeRotation _sm_oldbrickhouse_door_interior_01 (Math|Rotator|MakeRotator 0.0 0.0 _axisz) false false)
          (else
            (Transformation|SetRelativeRotation _sm_oldbrickhouse_door_interior_01 (Math|Rotator|MakeRotator 0.0 0.0 (- 1.0 _axisz)) false false)))))
    (else
      (Timeline|doorMovement Reverse))))

(fn ConstructionScript)