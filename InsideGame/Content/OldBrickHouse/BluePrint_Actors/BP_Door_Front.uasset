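; Front door actor that swings open and closed and shows a text prompt when the player is near.
; The MoveDoor event plays or reverses a timeline based on its AxisZ value, which sets the door mesh's relative yaw.
; IsOpeningInwards selects between that value and one minus it for the yaw.
; A box overlap toggles the TextRender's visibility for the ThirdPersonCharacter; MoveDoor has no caller in this graph.
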(event OnComponentEndOverlap(Box)
  (params (OverlappedComponent :type Primitive%20Component%20Object%20Reference) (OtherActor :type Actor%20Object%20Reference) (OtherComp :type Primitive%20Component%20Object%20Reference) (OtherBodyIndex :type Integer))
  (Utilities|Casting|CastToThirdPersonCharacter OtherActor)
  (Rendering|SetVisibility (Variables|Default|GetTextRender) false false))

(event OnComponentBeginOverlap(Box)
  (params (OverlappedComponent :type Primitive%20Component%20Object%20Reference) (OtherActor :type Actor%20Object%20Reference) (OtherComp :type Primitive%20Component%20Object%20Reference) (OtherBodyIndex :type Integer) (bFromSweep :type Boolean) (SweepResult :type Hit%20Result%20Structure%20%28by%20ref%29))
  (Utilities|Casting|CastToThirdPersonCharacter OtherActor)
  (Rendering|SetVisibility (Variables|Default|GetTextRender) true false))

(event Custom|Move%20Door
  (bind _sm_door_front (Variables|Default|GetSM_Door_Front))
  (if (< (stale _axisz) 1.0)
    (bind _axisz (Timeline|Timeline_0 Play)
      (:Update
        (if (Variables|Default|GetisOpeningInwards)
          (Transformation|SetRelativeRotation _sm_door_front (Math|Rotator|MakeRotator 0.0 0.0 _axisz) false false)
          (else
            (Transformation|SetRelativeRotation _sm_door_front (Math|Rotator|MakeRotator 0.0 0.0 (- 1.0 _axisz)) false false)))))
    (else
      (Timeline|Timeline_0 Reverse))))

(fn ConstructionScript)